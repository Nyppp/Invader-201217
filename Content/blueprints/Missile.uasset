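; Missile is a movable actor that follows the player while the player is within its PlayerFollow overlap area.
; Each Tick it checks whether any Ailen (alien) actor overlaps AilenStop; if so, it stops adding movement and shows its Arrow.
; Otherwise it hides the Arrow, moves toward the player at reduced input scale and copies the player's rotation rather than facing its travel direction.
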(event `self.ReceiveTick`
  (params (DeltaSeconds :type "Float (single-precision)"))
  (bind _returnvalue (`GameplayStatics.GetPlayerCharacter` 0))
  (bind _arrow (`self.Arrow`))
  (if (`PrimitiveComponent.IsOverlappingActor` (`self.Player_Follow`) _returnvalue)
    (set `self.Stop` (`KismetArrayLibrary.Array_IsValidIndex` (`PrimitiveComponent.GetOverlappingActors` (`self.Ailen_Stop`) "/Game/Ailen/Ailen.Ailen_C")))
    (if (`self.Stop`)
      (`SceneComponent.SetVisibility` _arrow true false)
      (else
        (`SceneComponent.SetVisibility` _arrow false false)
        (`self.AddMovementInput` (`KismetMathLibrary.Normal` (- (`self.K2_GetActorLocation` _returnvalue) (`self.K2_GetActorLocation`))) 0.7)
        (`self.K2_SetActorRotation` (* (`self.K2_GetActorRotation` _returnvalue) 1.0))))))

(fn `UserConstructionScript`)